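; Loot pickup actor with a rarity tier, shown by the material on its cube.
; On interact, it puts itself in the player's first empty HUD inventory slot, refreshes that slot, breaks the search via LootCollected and destroys the actor.
; The construction script derives Rarity from a RandomStat roll indexed into the Rarities array, then uses SetRarityMaterial to apply the matching material, from Useless to Cursed.
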(event Custom|LootCollected
  (Utilities|Array|ForEachLoopwithBreak (Variables|/Game/BrenonContent/PlayerCharacter/HUDWidgets/HUD.HUD_C|GetInventory (Variables|/Game/BrenonContent/PlayerCharacter/FirstPersonCharacter.FirstPersonCharacter_C|GetHUD (stale EventInteract Player)))) ; enters at Break
)

(event EventInteract
  (params (Player :type First%20Person%20Character%20Object%20Reference))
  (bind _array_element (Utilities|Array|ForEachLoopwithBreak (Variables|/Game/BrenonContent/PlayerCharacter/HUDWidgets/HUD.HUD_C|GetInventory (Variables|/Game/BrenonContent/PlayerCharacter/FirstPersonCharacter.FirstPersonCharacter_C|GetHUD Player)))
    (:LoopBody
      (if (Variables|/Game/BrenonContent/PlayerCharacter/HUDWidgets/InventorySlot.InventorySlot_C|GetEmpty _array_element)
        (Variables|/Game/BrenonContent/PlayerCharacter/HUDWidgets/InventorySlot.InventorySlot_C|SetItem _array_element self)
        (Variables|/Game/BrenonContent/PlayerCharacter/HUDWidgets/InventorySlot.InventorySlot_C|SetEmpty _array_element false)
        (Default|UpdateSlot _array_element)
        (CallFunction|LootCollected)
        (Actor|DestroyActor)))))

(fn ConstructionScript
  (bind _valueout (CallFunction|RandomStat "/Game/BrenonContent/Loot/Curves/Rarity.Rarity"))
  (bind _output_get (Variables|Default|SetRarity (Utilities|Array|Get(acopy) (Variables|Default|GetRarities) (/ (Math|Float|Round _valueout) 10))))
  (switch Utilities|FlowControl|Switch|SwitchonRarity _output_get
    (:NewEnumerator0
      (|SetRarityMaterial :!label _label))
    (:NewEnumerator1
      (goto _label Common))
    (:NewEnumerator2
      (goto _label Rare))
    (:NewEnumerator3
      (goto _label Epic))
    (:NewEnumerator4
      (goto _label Legendary))
    (:NewEnumerator5
      (goto _label Set))
    (:NewEnumerator6
      (goto _label Cursed))))