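; Loot chest actor that spawns random loot when its Interact event fires.
; Each offset in LootSpawns is rotated by the chest's rotation and added to its location, so spawn points follow the chest's placement.
; Every point gets a class picked from a hard-coded index range of the Loot array, spawned with shared LootRotation and LootScale.
; Nothing in the graph prevents repeated looting.
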(event EventInteract
  (params (Player :type First%20Person%20Character%20Object%20Reference))
  (for _array_element (Variables|Default|GetLootSpawns)
    (Game|SpawnActorfromClass (Utilities|Array|Get(acopy) (Variables|Default|GetLoot) (Math|Random|RandomIntegerinRange 0 7)) (Math|Transform|MakeTransform (+ (Math|Vector|RotateVector _array_element (Transformation|GetActorRotation)) (Transformation|GetActorLocation)) (Variables|Default|GetLootRotation) (Variables|Default|GetLootScale)) "Undefined" 0 0)))

(fn ConstructionScript)