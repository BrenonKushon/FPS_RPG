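; Ammo loot pickup that adds a rolled amount of ammo to the player who interacts with it.
; Construction sets the cube's Useless material, fixes rarity and loot type, and truncates a level-based random roll between min and max curves into the amount.
; On Interact it increases the player's current ammo, calls the player's ammo update with the new total, then destroys itself.
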(event EventInteract
  (params (Player :type First%20Person%20Character%20Object%20Reference))
  (bind _output_get (Variables|/Game/BrenonContent/PlayerCharacter/FirstPersonCharacter.FirstPersonCharacter_C|SetCurrentAmmo Player (+ (Variables|/Game/BrenonContent/PlayerCharacter/FirstPersonCharacter.FirstPersonCharacter_C|GetCurrentAmmo Player) (Variables|Default|GetAmmount))))
  (Default|CallUpdateCurrentAmmo Player _output_get)
  (Actor|DestroyActor))

(fn ConstructionScript
  (Rendering|Material|SetMaterial (Variables|Default|GetCube) 0 "/Game/BrenonContent/Loot/RarityMaterials/Useless.Useless")
  (Variables|Default|SetRarity "NewEnumerator0")
  (Variables|Default|SetLootType "NewEnumerator2")
  (bind _valueout (CallFunction|RandomStatbyLevel (Variables|Default|GetAmmountMin) (Variables|Default|GetAmmountMax)))
  (Variables|Default|SetAmmount (Math|Float|Truncate _valueout)))